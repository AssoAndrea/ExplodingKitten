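; An actor component that lets its owning character interact with objects in view and hold a cat for inspection.
; TryInteraction sphere-traces forward from the player camera and passes the hit actor through a server-named event, which sends it an interact message along with the component.
; InspectObject snaps a given actor to the third-person character's InspectPosition, sets its relative rotation and stores it as EquippedCat.
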(event `TryInteraction`
  (bind _returnvalue (`GameplayStatics.GetPlayerCameraManager` 0))
  (bind _returnvalue_2 (`PlayerCameraManager.GetCameraLocation` _returnvalue))
  (bind _outhit (`KismetSystemLibrary.SphereTraceSingle` _returnvalue_2 (+ _returnvalue_2 (* (`Actor.GetActorForwardVector` _returnvalue) (`self.InteractionDistance`))) (`self.InteractionRadius`) "TraceTypeQuery1"))
  (`self.Server_TryInteraction` (`.HitActor` (`GameplayStatics.BreakHitResult` _outhit)) self))

(event `Server_TryInteraction`
  (params (Target :type "Actor Object Reference") (InteractionComponent :type "/Game/Blueprints/Components/InteractionComponent Object Reference"))
  (message `/Game/Blueprints/Interfaces/Interactable.Interact` Target InteractionComponent))

(event `InspectObject`
  (params (ActorToInspect :type "Actor Object Reference") (InspectRotation :type "Rotator Structure"))
  (bind _asbp_third_person_character (cast `/Game/ThirdPerson/Blueprints/BP_ThirdPersonCharacter` (`self.GetOwner`) :!pure true))
  (`Actor.K2_AttachToComponent` ActorToInspect (`/Game/ThirdPerson/Blueprints/BP_ThirdPersonCharacter.InspectPosition` _asbp_third_person_character) "None" "SnapToTarget" "KeepWorld" "KeepRelative" true)
  (`Actor.K2_SetActorRelativeRotation` ActorToInspect InspectRotation false false)
  (set `/Game/ThirdPerson/Blueprints/BP_ThirdPersonCharacter.EquippedCat` (cast `/Game/Blueprints/Actors/BP_Cat` ActorToInspect :!pure true) _asbp_third_person_character))