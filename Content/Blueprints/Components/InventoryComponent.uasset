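; Inventory component for the third-person character that stores, switches, uses and drops weapons in a fixed number of slots.
; Picked-up types resolve through DT_Weapons into the first empty slot; the selected weapon is spawned and held through the InteractionComponent's inspect function.
; Dropping detaches the weapon with physics, and both dropping and using clear the slot.
; Multicast events replicate actions, CanUse blocks them while hidden, and OnEquipChange broadcasts inventory changes.
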(event `self.ReceiveBeginPlay`
  (bind _asbp_third_person_character (cast `/Game/ThirdPerson/Blueprints/BP_ThirdPersonCharacter` (`self.GetOwner`)))
  (bind _output_get (set `self.Owner_Ref` _asbp_third_person_character))
  (set `self.Mesh` (`Character.Mesh` _output_get))
  (set `self.Inspect Position` (`/Game/ThirdPerson/Blueprints/BP_ThirdPersonCharacter.InspectPosition` _output_get))
  (set `self.Interaction Component` (`/Game/ThirdPerson/Blueprints/BP_ThirdPersonCharacter.InteractionComponent` _asbp_third_person_character))
  (for _ (range (`self.MaxStack`))
    (`KismetArrayLibrary.Array_Add` (`self.Inventory`))))

(event `TakeItem`
  (params (Type :type "/Game/Blueprints/Actors/Weapon/E_WeaponType Enum" :default "NewEnumerator0"))
  ;[1 1 1] Add item to inventory
  (bind _returnvalue (`|GetDataTableRow` "/Game/Blueprints/Actors/Weapon/DT_Weapons.DT_Weapons" (`KismetStringLibrary.Conv_StringToName` (`|GetEnumeratorNameAsString` Type)))
    (:`then`
      (for (_array_element _array_index) (`self.Inventory`)
        (if (not (!= (`.WeaponClass_7_BA10B26248C506527C08F4A68F1380F8` (break `/Game/Blueprints/Actors/Weapon/S_WeaponData` _array_element)) null))
          (`KismetArrayLibrary.Array_Set` (`self.Inventory`) _array_index _returnvalue)
          (if (== (`self.currentIndex`) _array_index)
            (`self.EquipWeapon`)
            (break)
            (else
              (break)))))
      (`self.OnEquipChange` (`self.Inventory`) (`self.currentIndex`)))))

(event `SwitchWeapons`
  (params (B :type Integer))
  (bind _returnvalue (`KismetArrayLibrary.Array_Length` (`self.Inventory`)))
  ;[1 1 1] Switch Weapon
  (if (`self.CanUse`)
    (bind _output_get (set `self.currentIndex` (+ (stale _output_get) B)))
    (if (>= _output_get _returnvalue)
      (set `self.currentIndex` 0)
      (elif (< (`self.currentIndex`) 0)
        (set `self.currentIndex` (- _returnvalue 1))))
    (bind _currentweapon (`self.CurrentWeapon`)
      (:`then`
        (`Actor.K2_DestroyActor` _currentweapon)
        (set `self.CurrentWeapon` null))
      (:`else`
        _))
    (`self.EquipWeapon`)
    (`self.OnEquipChange` (`self.Inventory`) (`self.currentIndex`))))

(event `EquipWeapon`
  (bind (_name _weaponclass _image _socketname _rotationoffset) (break `/Game/Blueprints/Actors/Weapon/S_WeaponData` (`|GetArrayItem` (`self.Inventory`) (`self.currentIndex`))))
  ;[1 1 1] Equip Weapon
  (if (`KismetSystemLibrary.IsValidClass` _weaponclass)
    (bind _returnvalue (`|SpawnActorFromClass` _weaponclass (`KismetMathLibrary.MakeTransform` (0.0 0.0 0.0)) "Undefined" "MultiplyWithRoot" null null))
    (bind _output_get (set `self.CurrentWeapon` _returnvalue))
    (`self.Multi_EquipWeapon` _output_get _rotationoffset)))

(event `Multi_EquipWeapon`
  (params (`Actor To Inspet` :type "/Game/Blueprints/Actors/Weapon/BP_WeaponParent Object Reference") (InspectRotation :type "Rotator Structure"))
  ;[1 1 1] Equip Weapon
  (`/Game/Blueprints/Actors/Weapon/BP_WeaponParent.DisableCollision` `Actor To Inspet`)
  (`/Game/Blueprints/Components/InteractionComponent.InspectObject` (`self.Interaction Component`) `Actor To Inspet` InspectRotation))

(event `Drop`
  ;[1 1 1] Drop
  (`self.Multi_Drop`))

(event `Multi_Drop`
  (bind _currentweapon (`self.CurrentWeapon`))
  ;[1 1 1] Drop
  (if (`self.CanUse`)
    (`self.CurrentWeapon`
      (:`then`
        (`Actor.K2_DetachFromActor` (`self.CurrentWeapon`) "KeepWorld" "KeepWorld" "KeepWorld")
        (`Actor.SetActorEnableCollision` _currentweapon true)
        (`PrimitiveComponent.SetSimulatePhysics` (`StaticMeshActor.StaticMeshComponent` _currentweapon) true)
        (set `self.CurrentWeapon` null)
        (`KismetArrayLibrary.Array_Set` (`self.Inventory`) (`self.currentIndex`))
        (set `self.currentIndex` 0)
        (`self.OnEquipChange` (`self.Inventory`) (`self.currentIndex`)))
      (:`else`))))

(event `Use`
  ;[1 1 1] Use Weapon
  (if (`self.CanUse`)
    (`self.CurrentWeapon`
      (:`then`
        (`/Engine/EditorBlueprintResources/ActorComponentMacros.Switch Has Authority`
          (:`Authority`
            (`self.ServerToClientUse`))
          (:`Remote`
            (`self.ClientToSeverUse`))))
      (:`else`))))

(event `ServerToClientUse`
  ;[1 1 1] Use Weapon
  (`self.MulticastUse` :!label _label))

(event `MulticastUse`
  ;[1 1 1] Use Weapon
  (`/Game/Blueprints/Actors/Weapon/BP_WeaponParent.UseWeapon` (`self.CurrentWeapon`))
  (`KismetArrayLibrary.Array_Set` (`self.Inventory`) (`self.currentIndex`))
  (`self.OnEquipChange` (`self.Inventory`) (`self.currentIndex`)))

(event `ClientToSeverUse`
  ;[1 1 1] Use Weapon
  (goto _label))

(event `HideCurrentWeapon`
  (params (Hide :type Boolean))
  ;[1 1 1] HideCurrentWeapon
  (`self.RunOnServerHide` Hide))

(event `MultiHide`
  (params (Hide :type Boolean))
  ;[1 1 1] HideCurrentWeapon
  (bind _currentweapon (`self.CurrentWeapon`)
    (:`then`
      (`Actor.SetActorHiddenInGame` _currentweapon Hide)
      (set `self.CanUse` (not Hide)))
    (:`else`)))

(event `RunOnServerHide`
  (params (Hide :type Boolean))
  ;[1 1 1] HideCurrentWeapon
  (`self.MultiHide` Hide))