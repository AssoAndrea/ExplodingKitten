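; Game mode that runs a countdown from a configurable starting time.
; Tick accumulates delta time and calls Timer whenever it passes one second, resetting the accumulator to zero.
; Timer decrements the remaining time and broadcasts UpdateTimer with the new value.
; At zero or below it also broadcasts OnTimerEnd, which repeats on each later step because the countdown never stops.
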(event `self.ReceiveBeginPlay`
  (set `self.ActualTimer` (`self.StartingTimer`)))

(event `self.ReceiveTick`
  (params (DeltaSeconds :type "Float (single-precision)"))
  (bind _output_get (set `self.ProgressTimer` (+ DeltaSeconds (`self.ProgressTimer`))))
  (if (> _output_get 1.0)
    (set `self.ProgressTimer` 0.0)
    (`self.Timer`)))

(fn `Timer`
  (bind _output_get (set `self.ActualTimer` (- (`self.ActualTimer`) 1.0)))
  (`self.UpdateTimer` _output_get)
  (if (<= _output_get 0.0)
    (`self.OnTimerEnd`)))

(fn `UserConstructionScript`)