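; Player controller that switches between normal play and a cursor-driven mode for pressing bomb keypad buttons.
; The O key toggles the cursor, swapping mapping contexts and input modes.
; Interact input calls the character's interaction component, while clicks trace under the cursor and send a button's value to its owning bomb.
; It also requests a free bomb code from the game state on BeginPlay and has an event that decrements and prints the active bomb count.
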(event `self.ReceiveBeginPlay`
  (`WidgetBlueprintLibrary.SetInputMode_GameOnly` self)
  (set `self.bShowMouseCursor` false)
  (bind _asks_game_state (cast `/Game/Blueprints/KS_GameState` (`GameplayStatics.GetGameState`)))
  (`/Game/Blueprints/KS_GameState.GetFreeBombCode` _asks_game_state))

(event `Key|O`
  (params (Key :type "Key Structure"))
  (bind _returnvalue (pcsubsystem `EnhancedInputLocalPlayerSubsystem` self))
  (:`Pressed`
    (bind _output_get (set `self.bShowMouseCursor` (not (`self.bShowMouseCursor`))))
    (if _output_get
      (`EnhancedInputSubsystemInterface.RemoveMappingContext` _returnvalue "/Game/ThirdPerson/Input/IMC_Default.IMC_Default" (struct))
      (`EnhancedInputSubsystemInterface.AddMappingContext` _returnvalue "/Game/ThirdPerson/Input/IMC_BombInteraction.IMC_BombInteraction" 0 (struct))
      (`WidgetBlueprintLibrary.SetInputMode_GameAndUIEx` self null)
      (else
        (`EnhancedInputSubsystemInterface.AddMappingContext` _returnvalue "/Game/ThirdPerson/Input/IMC_Default.IMC_Default" 0 (struct))
        (`EnhancedInputSubsystemInterface.RemoveMappingContext` _returnvalue "/Game/ThirdPerson/Input/IMC_BombInteraction.IMC_BombInteraction" (struct))
        ;[1 1 1] To focus the window
        (`WidgetBlueprintLibrary.SetInputMode_GameOnly` self)))))

(event `EnhancedInput|/Game/ThirdPerson/Input/Actions/IA_Interact`
  (params (ActionValue :type Boolean) (ElapsedSeconds :type "Float (double-precision)") (TriggeredSeconds :type "Float (double-precision)") (InputAction :type "InputAction Object Reference" :default "/Game/ThirdPerson/Input/Actions/IA_Interact.IA_Interact"))
  (:`Triggered`
    (bind _asbp_third_person_character (cast `/Game/ThirdPerson/Blueprints/BP_ThirdPersonCharacter` (`self.K2_GetPawn`)))
    (`/Game/Blueprints/Components/InteractionComponent.TryInteraction` (`/Game/ThirdPerson/Blueprints/BP_ThirdPersonCharacter.InteractionComponent` _asbp_third_person_character))))

(event `EnhancedInput|/Game/ThirdPerson/Input/Actions/BombInteraction/IA_ClickButton`
  (params (ActionValue :type Boolean) (ElapsedSeconds :type "Float (double-precision)") (TriggeredSeconds :type "Float (double-precision)") (InputAction :type "InputAction Object Reference" :default "/Game/ThirdPerson/Input/Actions/BombInteraction/IA_ClickButton.IA_ClickButton"))
  (:`Triggered`
    (bind _asbp_button (cast `/Game/Blueprints/Actors/BP_Button` (`.HitActor` (`GameplayStatics.BreakHitResult` (`self.GetHitResultUnderCursorByChannel` "TraceTypeQuery1")))))
    (`/Game/Blueprints/Actors/BP_Bomb.OnBombNumberPressed` (`/Game/Blueprints/Actors/BP_Button.OwnerBomb` _asbp_button) (`/Game/Blueprints/Actors/BP_Button.ButtonValue` _asbp_button))))

(event `ChangeNumber`
  (bind _asks_game_state (cast `/Game/Blueprints/KS_GameState` (`GameplayStatics.GetGameState`)))
  (bind _result (`/Engine/EditorBlueprintResources/StandardMacros.DecrementInt` (`/Game/Blueprints/KS_GameState.Active Bombs` _asks_game_state))
    (:`  `
      (`KismetSystemLibrary.PrintString` (`KismetStringLibrary.Conv_IntToString` _result)))))

(fn `UserConstructionScript`)