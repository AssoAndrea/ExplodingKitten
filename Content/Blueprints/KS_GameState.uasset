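; Game state for a bomb-defusing match, handling the countdown, bomb codes, active bomb count and win or loss.
; Server init reads config amounts, then a multicast rolls random four-digit codes locally on each machine into bomb and cat pools.
; Authority Tick counts down each second once started, triggering game over at zero, while unarmed bombs reduce the count toward a win.
; Multicasts relay timer, defusal and end-of-match events to dispatchers.
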(event `self.ReceiveBeginPlay`)

(event `Init_GameState`
  (`self.Server_GenerateCodes`))

(event `Server_GenerateCodes`
  (bind _config (`/Game/Blueprints/Structures/SpawnConfigClass.Config` (`self.ConfigurationAsset`)))
  (`/Engine/EditorBlueprintResources/ActorMacros.Switch Has Authority`
    (:`Authority`
      (set `self.ActualTimer` (`self.StartingTimer`))
      (set `self.Active Bombs` (break `/Game/Blueprints/Structures/KittenSpawnStruct` (`BlueprintMapLibrary.Map_Find` _config "NewEnumerator0")))
      (set `self.GameEnded` false)
      (set `self.StartBombCodes` (break `/Game/Blueprints/Structures/KittenSpawnStruct` (`BlueprintMapLibrary.Map_Find` _config "NewEnumerator1")))
      (`self.Multi_GenerateCodes`))))

(event `RestartMatch`
  (`self.Server_RestartMatch`))

(event `Server_RestartMatch`
  (bind _asks_game_mode (cast `/Game/Blueprints/GameMode/KS_GameMode` (`GameplayStatics.GetGameMode`)))
  (`GameMode.RestartGame` _asks_game_mode))

(event `Multi_GenerateCodes`
  (bind _freebombcodes (`self.FreeBombCodes`))
  (for _ (range 1 (+ (`self.StartBombCodes`) 1))
    (`KismetArrayLibrary.Array_Add` _freebombcodes (make `/Game/Blueprints/Structures/BombCode` (`self.GenerateBombCode`)))
    (bind _output_get (set `self.UnusedBombCodes` _freebombcodes))
    (set `self.FreeCatCodes` _output_get)))

(event `self.ReceiveTick`
  (params (DeltaSeconds :type "Float (single-precision)"))
  (`/Engine/EditorBlueprintResources/ActorMacros.Switch Has Authority`
    (:`Authority`
      (if (and (`self.HasMatchStarted`) (not (`self.GameEnded`)) (`self.GameStarted`))
        (bind _output_get (set `self.ProgressTimer` (+ DeltaSeconds (`self.ProgressTimer`))))
        (if (> _output_get 1.0)
          (set `self.ProgressTimer` 0.0)
          (`self.Timer`))))))

(event `Multi_UpdateTimer`
  (params (NewTimer :type "Float (double-precision)"))
  (`self.UpdateTimer` NewTimer))

(event `OnBombUnarmed`
  (params (BombCode :type "/Game/Blueprints/Structures/BombCode Structure"))
  (bind _active_bombs (`self.Active Bombs`))
  (bind _result (`/Engine/EditorBlueprintResources/StandardMacros.DecrementInt` _active_bombs)
    (:`  `
      (`self.Multi_OnBombUnarmed` BombCode)
      (if (<= _result 0)
        (`self.WinGame`)
        (else
          (`KismetSystemLibrary.PrintString` (`KismetStringLibrary.Conv_IntToString` _active_bombs)))))))

(event `Multi_OnBombUnarmed`
  (params (BombCode :type "/Game/Blueprints/Structures/BombCode Structure"))
  (`self.BombUnarmed` BombCode))

(event `WinGame`
  (`self.Server_OnWinGame`))

(event `StartGame`
  (set `self.GameStarted` true))

(event `Server_OnWinGame`
  (`self.Multi_OnWinGame`)
  (set `self.GameEnded` true))

(event `Multi_OnWinGame`
  (`self.OnWinGame`))

(event `GameOver`
  (`self.Server_OnGameOver`))

(event `Server_OnGameOver`
  (`self.Multi_OnGameOver`)
  (set `self.GameEnded` true))

(event `Multi_OnGameOver`
  (`self.OnGameOver`))

(fn `GenerateBombCode`
  (returns (OutCode :type "Array of Integer"))
  (locals (Code :type "Array of Integer"))
  (for _ (range 4)
    (`KismetArrayLibrary.Array_Add` (`local.Code`) (`KismetMathLibrary.RandomIntegerInRange` 1 9)))
  (return (`local.Code`)))

(fn `GetFreeBombCode`
  (returns (Code :type "/Game/Blueprints/Structures/BombCode Structure"))
  (bind _freebombcodes (`self.FreeBombCodes`))
  (if (`KismetArrayLibrary.Array_IsNotEmpty` _freebombcodes)
    (`KismetArrayLibrary.Array_Remove` (`self.FreeBombCodes`))
    (return (`|GetArrayItem` _freebombcodes))))

(fn `GetFreeCatCode`
  (returns (Code :type "/Game/Blueprints/Structures/BombCode Structure"))
  (bind _freecatcodes (`self.FreeCatCodes`))
  (if (`KismetArrayLibrary.Array_IsNotEmpty` _freecatcodes)
    (`KismetArrayLibrary.Array_Remove` (`self.FreeCatCodes`))
    (return (`|GetArrayItem` _freecatcodes))))

(fn `Timer`
  (bind _output_get (set `self.ActualTimer` (- (`self.ActualTimer`) 1.0)))
  (`self.Multi_UpdateTimer` _output_get)
  (if (<= _output_get 0.0)
    (`self.OnTimerEnd`)
    (`self.GameOver`)))

(fn `UserConstructionScript`)