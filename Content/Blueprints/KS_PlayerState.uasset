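; KS_PlayerState is a player state that tracks the codes a player owns.
; On BeginPlay it binds to the code-acquired dispatcher on KS_PlayerController, then to the bomb-unarmed dispatcher on KS_GameState.
; Acquired codes are added to OwnedCodes, and an unarmed bomb's code is removed from it.
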(event `self.ReceiveBeginPlay`
  (bind _asks_player_controller (cast `/Game/Blueprints/KS_PlayerController` (`self.GetPlayerController`)))
  (add `/Game/Blueprints/KS_PlayerController.OnCodeAcquired` _asks_player_controller (delegate `OnCodeAcquired`))
  (bind _asks_game_state (cast `/Game/Blueprints/KS_GameState` (`GameplayStatics.GetGameState`)))
  (add `/Game/Blueprints/KS_GameState.BombUnarmed` _asks_game_state (delegate `BombUnarmed_Event`)))

(event `OnCodeAcquired`
  (params (Code :type "/Game/Blueprints/Structures/BombCode Structure"))
  (`KismetArrayLibrary.Array_Add` (`self.OwnedCodes`) Code))

(event `BombUnarmed_Event`
  (params (BombCode :type "/Game/Blueprints/Structures/BombCode Structure"))
  (`KismetArrayLibrary.Array_RemoveItem` (`self.OwnedCodes`) BombCode))

(fn `UserConstructionScript`)