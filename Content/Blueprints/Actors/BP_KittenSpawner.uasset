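; Actor that populates the level with kittens at random navmesh points within a spawn radius, which its construction script previews as a debug sphere.
; On BeginPlay it reads the GameState's configuration asset, and the server starts a short one-shot timer to spawn.
; It spawns each configured type's amount, then fills up to the total with default kittens, storing spawned actors in a map by type.
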(event `self.ReceiveBeginPlay`
  (bind _asks_game_state (cast `/Game/Blueprints/KS_GameState` (`GameplayStatics.GetGameState`)))
  (set `self.ConfigurationAsset` (`/Game/Blueprints/KS_GameState.ConfigurationAsset` _asks_game_state))
  (if (`KismetSystemLibrary.IsServer`)
    (`KismetSystemLibrary.K2_SetTimerDelegate` (delegate `SpawnKitten`) 3.0)))

(event `SpawnKitten`
  (`self.Server Spawn Kittens`))

(event `Server Spawn Kittens`
  (`self.Spawn Kittens`))

(fn `Spawn Kittens`
  (bind _configurationasset (`self.ConfigurationAsset`))
  (bind _spawnedkittens (`self.SpawnedKittens`))
  (bind _tempkittens (`self.TempKittens`))
  (bind _tempkittens_2 (`self.TempKittens`))
  (bind _config (`/Game/Blueprints/Structures/SpawnConfigClass.Config` _configurationasset))
  (bind _returnvalue (`GameplayStatics.GetActorOfClass` "/Script/NavigationSystem.RecastNavMesh"))
  (set `self.RecastNavMesh` _returnvalue)
  (bind _keys (`BlueprintMapLibrary.Map_Keys` _config))
  (for _array_element _keys
    (`KismetArrayLibrary.Array_Clear` (`self.TempKittens`))
    (bind _value (`BlueprintMapLibrary.Map_Find` _config _array_element))
    (for _ (range (break `/Game/Blueprints/Structures/KittenSpawnStruct` _value))
      (`/Engine/EditorBlueprintResources/StandardMacros.IncrementInt` (`self.SpawnedCounter`)
        (:`  `
          (bind (_randomlocation _returnvalue_2) (`NavigationSystemV1.K2_GetRandomLocationInNavigableRadius` (`self.K2_GetActorLocation`) (`self.SpawnRadius`) (`self.RecastNavMesh`) "/Script/NavigationSystem.RecastFilter_UseDefaultArea"))
          (if _returnvalue_2
            (bind _returnvalue_3 (`|SpawnActorFromClass` (`.BpToUse_8_96915FC24EF3BEECB1C32AAA17A8CF9D` (break `/Game/Blueprints/Structures/KittenSpawnStruct` _value)) (`KismetMathLibrary.MakeTransform` (+ _randomlocation (0.0 0.0 50.0))) "AdjustIfPossibleButAlwaysSpawn" "MultiplyWithRoot" null null))
            (`KismetArrayLibrary.Array_Add` _tempkittens_2 _returnvalue_3)))))
    (`BlueprintMapLibrary.Map_Add` _spawnedkittens _array_element (make `/Game/Blueprints/Structures/ListOfKittens` _tempkittens_2)))
  (`KismetArrayLibrary.Array_Clear` _tempkittens)
  (for _ (range (- (`/Game/Blueprints/Structures/SpawnConfigClass.TotalKittens` _configurationasset) (`self.SpawnedCounter`)))
    (bind _randomlocation_2 (`NavigationSystemV1.K2_GetRandomLocationInNavigableRadius` (`self.K2_GetActorLocation`) (`self.SpawnRadius`) (`self.RecastNavMesh`) "/Script/NavigationSystem.RecastFilter_UseDefaultArea"))
    (bind _returnvalue_4 (`|SpawnActorFromClass` (`/Game/Blueprints/Structures/SpawnConfigClass.DefaultKitten` _configurationasset) (`KismetMathLibrary.MakeTransform` _randomlocation_2) "AdjustIfPossibleButAlwaysSpawn" "MultiplyWithRoot" null null))
    (`KismetArrayLibrary.Array_Add` _tempkittens_2 _returnvalue_4))
  (`BlueprintMapLibrary.Map_Add` _spawnedkittens "NewEnumerator7" (make `/Game/Blueprints/Structures/ListOfKittens` _tempkittens)))

(fn `UserConstructionScript`
  (`KismetSystemLibrary.DrawDebugSphere` (`self.K2_GetActorLocation`) (`self.SpawnRadius`) 12 (struct :`R` 1.0 :`G` 0.271568 :`A` 1.0) 1.0))