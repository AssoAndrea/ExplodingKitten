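; BP_StartGate is a gate actor that lowers into the ground when opened, likely to release players at a start point.
; It caches its location on BeginPlay, and OpenGate plays a Timeline that subtracts a Z offset from that position using teleporting moves.
; ServerOpenGate calls MultiOpenGate, which runs OpenGate, suggesting a server-to-multicast RPC chain so every client animates the gate.
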(event `self.ReceiveBeginPlay`
  (set `self.StartLocation` (`self.K2_GetActorLocation`)))

(event `ServerOpenGate`
  (`self.MultiOpenGate`))

(event `MultiOpenGate`
  (`self.OpenGate`))

(event `OpenGate`
  (bind (_startlocation_x _startlocation_y _startlocation_z) (`KismetMathLibrary.BreakVector` (`self.StartLocation`)))
  (bind (_direction _z) (`Timeline|Timeline`)
    (:`Update`
      (`self.K2_SetActorLocation` (`KismetMathLibrary.MakeVector` _startlocation_x _startlocation_y (- _startlocation_z _z)) false true))))

(fn `UserConstructionScript`)