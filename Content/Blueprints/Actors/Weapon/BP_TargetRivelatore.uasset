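; BP_TargetRivelatore is a one-use detector weapon that flags a nearby exploding cat.
; UseWeapon runs a wide Visibility sphere trace around itself and collects hit BP_ExplodingCat actors into BombKats.
; FindClosestCat is meant to pick the nearest, but compares distance against zero, so it effectively keeps the first.
; That cat shows its flag (ShowBandiera), then radar effects activate and the actor destroys itself after a short delay.
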(event `self.UseWeapon`
  (bind _returnvalue (`self.K2_GetActorLocation`))
  (bind (_outhits _returnvalue_2) (`KismetSystemLibrary.SphereTraceMulti` _returnvalue _returnvalue 2000.0 "TraceTypeQuery1"))
  (if _returnvalue_2
    (for _array_element _outhits
      (bind _asbp_exploding_cat (cast `/Game/Blueprints/Actors/Gatti/BP_ExplodingCat` (`.HitActor` (`GameplayStatics.BreakHitResult` _array_element))))
      (`KismetArrayLibrary.Array_Add` (`self.BombKats`) _asbp_exploding_cat))
    (`|ExecutionSequence`
      (:`then_0`
        (bind _cat (`self.FindClosestCat`))
        (`/Engine/EditorBlueprintResources/StandardMacros.IsValid` _cat
          (:`Is Valid`
            (`/Game/Blueprints/Actors/Gatti/BP_ExplodingCat.ShowBandiera` _cat))))
      (:`then_1`
        (`ActorComponent.Activate` (`self.NS_Radar`) false)
        (`ActorComponent.Activate` (`self.NS_Radar1`) false)
        (`KismetSystemLibrary.Delay` 2.0)
        (`self.K2_DestroyActor`)))))

(fn `FindClosestCat`
  (returns (Cat :type "/Game/Blueprints/Actors/Gatti/BP_ExplodingCat Object Reference"))
  (locals (distance :type "Float (double-precision)") (CatToFlag :type "Actor Object Reference"))
  (for (_array_element _array_index) (`self.BombKats`)
    (if (== _array_index 0)
      (set `local.CatToFlag` _array_element)
      (bind _returnvalue (`KismetMathLibrary.Vector_Distance` (`self.K2_GetActorLocation` _array_element) (`self.K2_GetActorLocation`)))
      (set `local.distance` _returnvalue)
      (elif (< _returnvalue 0.0)
        (set `local.distance` _returnvalue)
        (set `local.CatToFlag` _array_element))))
  (bind _asbp_exploding_cat (cast `/Game/Blueprints/Actors/Gatti/BP_ExplodingCat` (`local.CatToFlag`)))
  (return _asbp_exploding_cat))

(fn `UserConstructionScript`
  (`parent.UserConstructionScript`))