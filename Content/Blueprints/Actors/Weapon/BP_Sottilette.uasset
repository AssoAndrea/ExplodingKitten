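; BP_Sottilette is a throwable cheese-slice weapon that stuns a cat on impact.
; UseWeapon detaches it, enables collision and physics, and applies a forward force with a slight upward component.
; On the first hit after use, it hides the mesh and runs a debug-drawn sphere trace to call StunnedCat on a nearby BP_Cat.
; The actor destroys itself after a delay.
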(event `self.ReceiveBeginPlay`
  (`parent.ReceiveBeginPlay`)
  (`self.SetActorTickEnabled` false))

(event `self.UseWeapon`
  (bind (_returnvalue_x _returnvalue_y _returnvalue_z) (`KismetMathLibrary.BreakVector` (* (`self.GetActorForwardVector`) 500.0)))
  (set `self.CanCollide` true)
  (`KismetSystemLibrary.PrintString` "Sono la sottiletta")
  (`self.SetActorEnableCollision` true)
  (`PrimitiveComponent.SetSimulatePhysics` (`self.StaticMeshComponent`) true)
  (`self.K2_DetachFromActor` "KeepWorld" "KeepWorld" "KeepWorld")
  (`PrimitiveComponent.AddForce` (`self.StaticMeshComponent`) (+ (`KismetMathLibrary.MakeVector` _returnvalue_x _returnvalue_y _returnvalue_z) (0.0 0.0 100.0)) "None" false)
  (`self.SetActorTickEnabled` true))

(event `self.StaticMeshComponent.OnComponentHit`
  (params (HitComponent :type "PrimitiveComponent Object Reference") (OtherActor :type "Actor Object Reference") (OtherComp :type "PrimitiveComponent Object Reference") (NormalImpulse :type "Vector Structure") (Hit :type "HitResult Structure (by ref)"))
  (bind _returnvalue (`self.K2_GetActorLocation`))
  (if (`self.CanCollide`)
    (`SceneComponent.SetVisibility` (`self.StaticMeshComponent`) false false)
    (set `self.CanCollide` false)
    (bind _outhits (`KismetSystemLibrary.SphereTraceMulti` :`Start` _returnvalue :`End` _returnvalue :`Radius` 100.0 :`TraceChannel` "TraceTypeQuery1" :`DrawDebugType` "ForDuration"))
    (for _array_element _outhits
      (bind _asbp_cat (cast `/Game/Blueprints/Actors/BP_Cat` (`.HitActor` (`GameplayStatics.BreakHitResult` _array_element))))
      (`/Game/Blueprints/Actors/BP_Cat.StunnedCat` _asbp_cat)
      (break))
    (`KismetSystemLibrary.Delay` 10.0)
    (`self.K2_DestroyActor`)))

(fn `UserConstructionScript`
  (`parent.UserConstructionScript`))