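; BP_Cetrioli is a throwable cucumber weapon that scares nearby cats on impact.
; Using it detaches the actor, enables collision and physics, and launches it forward and upward with a velocity-change impulse.
; Once thrown, a component hit runs a multi-sphere trace around it and calls ScareTheCat on hit BP_Cat actors, passing its location.
; The cucumber destroys itself only when that trace reports a hit.
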(event `self.ReceiveBeginPlay`
  (`parent.ReceiveBeginPlay`)
  (`self.SetActorTickEnabled` false))

(event `self.UseWeapon`
  (bind (_returnvalue_x _returnvalue_y) (`KismetMathLibrary.BreakVector` (* (`self.GetActorForwardVector`) 500.0)))
  (set `self.CanCollide` true)
  (`KismetSystemLibrary.PrintString` "Sono il Cetriolo")
  (`self.SetActorEnableCollision` true)
  (`PrimitiveComponent.SetSimulatePhysics` (`self.StaticMeshComponent`) true)
  (`self.K2_DetachFromActor` "KeepWorld" "KeepWorld" "KeepWorld")
  (`PrimitiveComponent.AddImpulse` (`self.StaticMeshComponent`) (`KismetMathLibrary.MakeVector` _returnvalue_x _returnvalue_y 500.0) "None" true)
  (`self.SetActorTickEnabled` true))

(event `self.StaticMeshComponent.OnComponentHit`
  (params (HitComponent :type "PrimitiveComponent Object Reference") (OtherActor :type "Actor Object Reference") (OtherComp :type "PrimitiveComponent Object Reference") (NormalImpulse :type "Vector Structure") (Hit :type "HitResult Structure (by ref)"))
  (bind _returnvalue (`self.K2_GetActorLocation`))
  (if (`self.CanCollide`)
    (bind (_outhits _returnvalue_2) (`KismetSystemLibrary.SphereTraceMulti` :`Start` _returnvalue :`End` _returnvalue :`Radius` 400.0 :`TraceChannel` "TraceTypeQuery1" :`DrawDebugType` "ForDuration"))
    (if _returnvalue_2
      (for _array_element _outhits
        (bind _asbp_cat (cast `/Game/Blueprints/Actors/BP_Cat` (`.HitActor` (`GameplayStatics.BreakHitResult` _array_element))))
        (`/Game/Blueprints/Actors/BP_Cat.ScareTheCat` _asbp_cat (`self.K2_GetActorLocation`)))
      (`self.K2_DestroyActor`))))

(fn `UserConstructionScript`
  (`parent.UserConstructionScript`))