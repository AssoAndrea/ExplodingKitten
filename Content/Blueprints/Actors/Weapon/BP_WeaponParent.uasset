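; BP_WeaponParent is a base weapon actor that can be picked up through interaction.
; Interact finds the InventoryComponent on the interacting component's owner, calls TakeItem with the weapon's Type, then destroys the actor.
; UseWeapon is an empty event, and DisableCollision passes through server and multicast events to turn off actor collision across the network.
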(event `UseWeapon`)

(event `/Game/Blueprints/Interfaces/Interactable.Interact`
  (params (InteractionComponent :type "/Game/Blueprints/Components/InteractionComponent Object Reference"))
  (`/Game/Blueprints/Components/InventoryComponent.TakeItem` (`self.GetComponentByClass` (`ActorComponent.GetOwner` InteractionComponent) "/Game/Blueprints/Components/InventoryComponent.InventoryComponent_C") (`self.Type`))
  (`self.K2_DestroyActor`))

(event `DisableCollision`
  (`self.Server_DisableCollision`))

(event `Server_DisableCollision`
  (`self.Multi_DisableCollision`))

(event `Multi_DisableCollision`
  (`self.SetActorEnableCollision` false))

(fn `UserConstructionScript`)