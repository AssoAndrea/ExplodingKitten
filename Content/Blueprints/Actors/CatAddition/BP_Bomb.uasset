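; A keypad bomb actor linked to a cat, disarmed through spawned buttons.
; On BeginPlay the authority spawns an attached BP_Button at each Cube socket, using socket names for digit values or OK/NO special buttons.
; Digits fill a four-entry code, but OK never validates it: a full code, like the delete event, destroys the Cat and notifies KS_GameState of disarming.
; DestroyBomb removes the bomb and its attached actors.
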(event `self.ReceiveBeginPlay`
  (bind _cube (`self.Cube`))
  (`/Engine/EditorBlueprintResources/ActorMacros.Switch Has Authority`
    (:`Authority`
      (for _array_element (`SceneComponent.GetAllSocketNames` _cube)
        (`|ExecutionSequence`
          (:`then_0`
            (bind _returnvalue (`|SpawnActorFromClass` "/Game/Blueprints/Actors/CatAddition/BP_Button.BP_Button_C" (`SceneComponent.GetSocketTransform` _cube _array_element "RTS_World") "Undefined" "MultiplyWithRoot" null null))
            (`self.K2_AttachToActor` _returnvalue self "None" "KeepWorld" "SnapToTarget" "KeepWorld" true)
            (set `/Game/Blueprints/Actors/CatAddition/BP_Button.OwnerBomb` self _returnvalue))
          (:`then_1`
            (switch `name` _array_element
              (:`Default`
                (set `/Game/Blueprints/Actors/CatAddition/BP_Button.ButtonValue` (`KismetStringLibrary.Conv_StringToInt` (`KismetStringLibrary.Conv_NameToString` _array_element)) _returnvalue))
              (:`OK`
                (set `/Game/Blueprints/Actors/CatAddition/BP_Button.IsOkButton` true _returnvalue)
                (set `/Game/Blueprints/Actors/CatAddition/BP_Button.IsSpecialButton` true _returnvalue))
              (:`NO`
                (set `/Game/Blueprints/Actors/CatAddition/BP_Button.IsSpecialButton` false _returnvalue)
                (set `/Game/Blueprints/Actors/CatAddition/BP_Button.IsSpecialButton` true _returnvalue)))))))))

(event `OnBombNumberPressed`
  (params (Number :type Integer))
  (bind _currentcode (`self.CurrentCode`))
  (if (not (>= (`KismetArrayLibrary.Array_Length` _currentcode) 4))
    (`KismetArrayLibrary.Array_Add` _currentcode Number)
    (`KismetSystemLibrary.PrintString` (`KismetStringLibrary.Conv_IntToString` Number) true true (struct :`R` 1.0 :`G` 0.067224 :`A` 1.0))))

(event `OnDelButtonPressed`
  (`self.K2_DestroyActor` (`self.Cat`) :!label _label)
  (bind _asks_game_state (cast `/Game/Blueprints/KS_GameState` (`GameplayStatics.GetGameState`)))
  (`/Game/Blueprints/KS_GameState.OnBombUnarmed` _asks_game_state))

(event `OnOkButtonPressed`
  (if (>= (`KismetArrayLibrary.Array_Length` (`self.CurrentCode`)) 4)
    (if true
      (goto _label)
      (else
        (`KismetSystemLibrary.PrintString` "SBAGLIATO")))))

(fn `DestroyBomb`
  (bind (_arrayindex _arrayelement) (`/Engine/EditorBlueprintResources/StandardMacros.ReverseForEachLoop` (`self.GetAttachedActors` true true))
    (:`LoopBody`
      (`self.K2_DestroyActor` _arrayelement))
    (:`Completed`
      (`self.K2_DestroyActor`))))

(fn `GetBombAsString`
  (returns (OutCodeAsString :type String))
  (locals (CodeAsString :type String))
  (for _array_element _
    (set `local.CodeAsString` (`KismetStringLibrary.Concat_StrStr` (`local.CodeAsString`) (`KismetStringLibrary.Conv_IntToString` _array_element))))
  (return (`local.CodeAsString`)))

(fn `UserConstructionScript`)