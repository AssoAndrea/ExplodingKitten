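; Duck variant of a usable cat actor that shows its Duck component on interaction and hides it when dropped.
; Using it triggers a duck-rain Niagara effect above the actor through a server-to-multicast event, plus a quack sound.
; It then hides its meshes in a random smoke puff, swaps the local player's cat interaction input context for the normal one and destroys itself after a short delay.
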(event `Multi_SpawnNiagara`
  (`NiagaraFunctionLibrary.SpawnSystemAtLocation` "/Game/Vfx/RainDuck/NS_RainDuck.NS_RainDuck" (+ (`self.K2_GetActorLocation`) (0.0 0.0 500.0))))

(event `Server_SpawnNiagara`
  (`self.Multi_SpawnNiagara`))

(event `self.UseCat`
  (params (Controller :type "/Game/Blueprints/KS_PlayerController Object Reference"))
  (bind _returnvalue (pcsubsystem `EnhancedInputLocalPlayerSubsystem` Controller))
  (`parent.UseCat` Controller)
  (`|ExecutionSequence`
    (:`then_0`
      (`self.Server_SpawnNiagara`))
    (:`then_1`
      (`GameplayStatics.PlaySoundAtLocation` "/Game/Audio/QuackRain.QuackRain" (`self.K2_GetActorLocation`) (struct) 1.0 1.0 0.0 null null null null)
      (`SceneComponent.SetVisibility` (`self.StaticMesh_0`) false false)
      (`SceneComponent.SetVisibility` (`self.duck`) false false)
      (`self.Puff`)
      (if (`Controller.IsLocalController` Controller)
        (`EnhancedInputSubsystemInterface.RemoveMappingContext` _returnvalue "/Game/ThirdPerson/Input/IMC_CatInteraction.IMC_CatInteraction" (struct))
        (`EnhancedInputSubsystemInterface.AddMappingContext` _returnvalue "/Game/ThirdPerson/Input/IMC_Interaction.IMC_Interaction" 0 (struct)))
      (`KismetSystemLibrary.Delay` 1.0)
      (`self.K2_DestroyActor`))))

(event `/Game/Blueprints/Interfaces/Interactable.Interact`
  (params (InteractionComponent :type "/Game/Blueprints/Components/InteractionComponent Object Reference"))
  (`parent.Interact` InteractionComponent)
  (`SceneComponent.SetVisibility` (`self.duck`) true false))

(event `self.OnCatDropped`
  (`parent.OnCatDropped`)
  (`SceneComponent.SetVisibility` (`self.duck`) false false))

(event `Puff`
  (`SceneComponent.SetVisibility` (`self.Mesh`) false false)
  (`NiagaraFunctionLibrary.SpawnSystemAttached` (`KismetArrayLibrary.Array_Random` (`|MakeArray` "/Game/Vfx/01-Smoke/NS_Smoke.NS_Smoke" "/Game/Vfx/01-Smoke/NS_Smoke_Ver2.NS_Smoke_Ver2" :!type "NiagaraSystem Object Reference")) (`self.Mesh`) "None" (0.0 0.0 0.0) (struct) "SnapToTarget"))

(fn `UserConstructionScript`
  (`parent.UserConstructionScript`))