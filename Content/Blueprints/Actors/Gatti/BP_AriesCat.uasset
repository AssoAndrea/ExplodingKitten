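; BP_AriesCat is an AI cat that wanders, chases nearby player characters and knocks them away on contact.
; Tick runs its state: Walking moves to random reachable points with random pauses, while Custom follows the target via AIMoveTo.
; SearchTarget uses a sphere overlap to set or clear the target and switch states, likely driven by BeginPlay's looping timer.
; Capsule hits apply a velocity-change impulse away from the cat, with halved vertical strength.
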(event `self.ReceiveBeginPlay`
  (`parent.ReceiveBeginPlay`)
  (`self.ChangeState` "NewEnumerator2")
  (`KismetSystemLibrary.K2_SetTimerDelegate` (`|CreateDelegate` :!event `SearchTarget`) 0.5 true))

(event `ChangeState`
  (params (NewState :type "/Game/Blueprints/Structures/KittenStatus Enum" :default "NewEnumerator0"))
  (bind _output_get (set `self.CurrentStatus` NewState))
  (switch `/Game/Blueprints/Structures/KittenStatus` _output_get
    (:`NewEnumerator2`
      (`self.WalkAround`)
      (set `self.MoveComplete` false))
    (:`NewEnumerator4`
      (`self.Chase`))))

(event `WalkAround`
  (if (`self.MoveComplete`)
    (set `self.MoveComplete` false)
    (`|AIMoveTo` self (`NavigationSystemV1.K2_GetRandomReachablePointInRadius` (`self.K2_GetActorLocation`) 1000.0 null "/Script/NavigationSystem.RecastFilter_UseDefaultArea") null 20.0
      (:`OnSuccess`
        _)
      (:`OnFail`
        _))
    (if true
      (`KismetSystemLibrary.Delay` (`KismetMathLibrary.RandomFloatInRange` 1.0 3.0))
      (set `self.MoveComplete` true))))

(event `/Game/Blueprints/Interfaces/Interactable.Interact`
  (params (InteractionComponent :type "/Game/Blueprints/Components/InteractionComponent Object Reference")))

(event `self.ReceiveTick`
  (params (DeltaSeconds :type "Float (single-precision)"))
  (switch `/Game/Blueprints/Structures/KittenStatus` (`self.CurrentStatus`)
    (:`NewEnumerator2`
      (`self.WalkAround`))
    (:`NewEnumerator4`
      (`self.Chase`))))

(event `Chase`
  (`|AIMoveTo` self (0.0 0.0 0.0) (`self.Target Actor`)))

(event `self.CapsuleComponent.OnComponentHit`
  (params (HitComponent :type "PrimitiveComponent Object Reference") (OtherActor :type "Actor Object Reference") (OtherComp :type "PrimitiveComponent Object Reference") (NormalImpulse :type "Vector Structure") (Hit :type "HitResult Structure (by ref)"))
  (bind _asbp_third_person_character (cast `/Game/ThirdPerson/Blueprints/BP_ThirdPersonCharacter` OtherActor))
  (`CharacterMovementComponent.AddImpulse` (`Character.CharacterMovement` _asbp_third_person_character) (* (`KismetMathLibrary.Normal` (- (`self.K2_GetActorLocation` OtherActor) (`self.K2_GetActorLocation`))) (`self.ImpulseStrenght`) (1.0 1.0 0.5)) true))

(event `SearchTarget`
  (bind (_outactors _returnvalue) (`KismetSystemLibrary.SphereOverlapActors` (`self.K2_GetActorLocation`) (`self.SearchRadius`) (`|MakeArray` "ObjectTypeQuery3" :!type "EObjectTypeQuery Enum") "/Game/ThirdPerson/Blueprints/BP_ThirdPersonCharacter.BP_ThirdPersonCharacter_C"))
  (if _returnvalue
    (if (not (`KismetArrayLibrary.Array_Contains` _outactors (`self.Target Actor`)))
      (set `self.Target Actor` (`|GetArrayItem` _outactors))
      (`self.ChangeState` "NewEnumerator4"))
    (elif (`|EnumEquality` (`self.CurrentStatus`) "NewEnumerator4")
      (`self.ChangeState` "NewEnumerator2")
      (set `self.Target Actor` null))))

(fn `UserConstructionScript`
  (`parent.UserConstructionScript`))