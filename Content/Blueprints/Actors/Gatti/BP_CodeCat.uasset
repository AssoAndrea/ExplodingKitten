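; BP_CodeCat is a cat variant that carries a bomb code for the player who uses it.
; On BeginPlay the server claims a free code from KS_GameState and copies it into a BP_Code child actor, or destroys the cat if none remains.
; Interacting reveals that child through Multi_Interact, and dropping hides it.
; Using the cat grants the code, spawns random smoke, destroys it and restores the local interaction input context.
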(event `self.UseCat`
  (params (Controller :type "/Game/Blueprints/KS_PlayerController Object Reference"))
  (bind _returnvalue (pcsubsystem `EnhancedInputLocalPlayerSubsystem` Controller))
  ;[1 0.4551 0.05415] Use Cat
  (`parent.UseCat` Controller)
  (`/Game/Blueprints/KS_PlayerController.AcquireCode` Controller (`self.BombCode`))
  (`NiagaraFunctionLibrary.SpawnSystemAtLocation` (`KismetArrayLibrary.Array_Random` (`|MakeArray` "/Game/Vfx/01-Smoke/NS_Smoke.NS_Smoke" "/Game/Vfx/01-Smoke/NS_Smoke_Ver2.NS_Smoke_Ver2" :!type "NiagaraSystem Object Reference")) (`self.K2_GetActorLocation`))
  (`self.K2_DestroyActor`)
  (if (`Controller.IsLocalController` Controller)
    (`EnhancedInputSubsystemInterface.RemoveMappingContext` _returnvalue "/Game/ThirdPerson/Input/IMC_CatInteraction.IMC_CatInteraction" (struct))
    (`EnhancedInputSubsystemInterface.AddMappingContext` _returnvalue "/Game/ThirdPerson/Input/IMC_Interaction.IMC_Interaction" 0 (struct))))

(event `self.ReceiveBeginPlay`
  (`parent.ReceiveBeginPlay`)
  (`SceneComponent.SetVisibility` (`self.ChildActor`) false true)
  (if (`KismetSystemLibrary.IsServer`)
    (bind _asks_game_state (cast `/Game/Blueprints/KS_GameState` (`GameplayStatics.GetGameState`)))
    (bind _code (`/Game/Blueprints/KS_GameState.GetFreeCatCode` _asks_game_state))
    (bind _string (`/Game/Blueprints/Library/Utils.ConvertCodeToString` _code))
    (if (`KismetStringLibrary.IsEmpty` _string)
      (`self.K2_DestroyActor`)
      (else
        (bind _output_get (set `self.BombCode` _code))
        (bind _asbp_code (cast `/Game/Blueprints/Actors/CatAddition/BP_Code` (`ChildActorComponent.ChildActor` (`self.ChildActor`))))
        (set `/Game/Blueprints/Actors/CatAddition/BP_Code.Code` _output_get _asbp_code)))))

(event `/Game/Blueprints/Interfaces/Interactable.Interact`
  (params (InteractionComponent :type "/Game/Blueprints/Components/InteractionComponent Object Reference"))
  (`parent.Interact` InteractionComponent)
  (`self.Multi_Interact`))

(event `Multi_Interact`
  (`SceneComponent.SetVisibility` (`self.ChildActor`) true true))

(event `self.OnCatDropped`
  (`parent.OnCatDropped`)
  (`SceneComponent.SetVisibility` (`self.ChildActor`) false true))

(fn `UserConstructionScript`
  (`parent.UserConstructionScript`))