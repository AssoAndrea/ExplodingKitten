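; Wizard cat variant of a usable cat actor, showing a magic wand mesh on interaction via multicast and hiding it when dropped.
; When used, the server traces down from a point ahead of the player's pawn and spawns a BP_Portal above the hit point.
; The cat then vanishes in random smoke, restores the local player's normal interaction input context and destroys itself after a short delay.
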(event `Multi_ShowMagicWand`
  (`SceneComponent.SetVisibility` (`self.StaticMesh`) true false))

(event `/Game/Blueprints/Interfaces/Interactable.Interact`
  (params (InteractionComponent :type "/Game/Blueprints/Components/InteractionComponent Object Reference"))
  (`parent.Interact` InteractionComponent)
  (`self.Multi_ShowMagicWand`))

(event `self.OnCatDropped`
  (`parent.OnCatDropped`)
  (`SceneComponent.SetVisibility` (`self.StaticMesh`) false false))

(event `self.UseCat`
  (params (Controller :type "/Game/Blueprints/KS_PlayerController Object Reference"))
  (bind _returnvalue (`Controller.K2_GetPawn` Controller))
  (bind _returnvalue_2 (pcsubsystem `EnhancedInputLocalPlayerSubsystem` Controller))
  (bind _returnvalue_3 (+ (`self.K2_GetActorLocation` _returnvalue) (* (`self.GetActorForwardVector` _returnvalue) 500.0)))
  (`parent.UseCat` Controller)
  (`|ExecutionSequence`
    (:`then_0`
      (if (`KismetSystemLibrary.IsServer`)
        (bind _outhit (`KismetSystemLibrary.LineTraceSingle` _returnvalue_3 (+ _returnvalue_3 (0.0 0.0 -500.0)) "TraceTypeQuery1"))
        (`|SpawnActorFromClass` "/Game/Blueprints/Actors/BP_Portal.BP_Portal_C" (`KismetMathLibrary.MakeTransform` (+ (`.ImpactPoint` (`GameplayStatics.BreakHitResult` _outhit)) (0.0 0.0 200.0)) (struct :`Yaw` 90.0)) "Undefined" "MultiplyWithRoot" null null)))
    (:`then_1`
      (`self.Puff`)
      (if (`Controller.IsLocalController` Controller)
        (`EnhancedInputSubsystemInterface.RemoveMappingContext` _returnvalue_2 "/Game/ThirdPerson/Input/IMC_CatInteraction.IMC_CatInteraction" (struct))
        (`EnhancedInputSubsystemInterface.AddMappingContext` _returnvalue_2 "/Game/ThirdPerson/Input/IMC_Interaction.IMC_Interaction" 0 (struct)))
      (`KismetSystemLibrary.Delay` 1.0)
      (`self.K2_DestroyActor`))))

(event `Puff`
  (`SceneComponent.SetVisibility` (`self.Mesh`) false false)
  (`NiagaraFunctionLibrary.SpawnSystemAttached` (`KismetArrayLibrary.Array_Random` (`|MakeArray` "/Game/Vfx/01-Smoke/NS_Smoke.NS_Smoke" "/Game/Vfx/01-Smoke/NS_Smoke_Ver2.NS_Smoke_Ver2" :!type "NiagaraSystem Object Reference")) (`self.Scene`) "None" (0.0 0.0 0.0) (struct) "SnapToTarget"))

(fn `UserConstructionScript`
  (`parent.UserConstructionScript`))