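; BP_GattoItem is an interactable cat actor that grants an item when used.
; Its static mesh starts hidden and is revealed through a Multi event on Interact.
; UseCat passes the item type to the pawn's InventoryComponent via a Server event, plays puff feedback and hides both meshes.
; It then restores the local player's normal interaction input context in place of the cat one and destroys itself after a short delay.
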(event `self.ReceiveBeginPlay`
  (`parent.ReceiveBeginPlay`)
  (`SceneComponent.SetVisibility` (`self.StaticMesh`) false false))

(event `Server_TakeItem`
  (params (Target :type "/Game/Blueprints/Components/InventoryComponent Object Reference"))
  (`/Game/Blueprints/Components/InventoryComponent.TakeItem` Target (`self.ItemType`)))

(event `self.UseCat`
  (params (Controller :type "/Game/Blueprints/KS_PlayerController Object Reference"))
  (bind _returnvalue (pcsubsystem `EnhancedInputLocalPlayerSubsystem` Controller))
  (`parent.UseCat` Controller)
  (`|ExecutionSequence`
    (:`then_0`
      (`self.Server_TakeItem` (`self.GetComponentByClass` (`Controller.K2_GetPawn` Controller) "/Game/Blueprints/Components/InventoryComponent.InventoryComponent_C"))
      (`GameplayStatics.PlaySound2D` "/Game/Audio/Puff.Puff" 1.0 1.0 0.0 null null))
    (:`then_1`
      (`self.Puff`)
      (`SceneComponent.SetVisibility` (`self.Mesh`) false false)
      (`SceneComponent.SetVisibility` (`self.StaticMesh`) false false)
      (if (`Controller.IsLocalController` Controller)
        (`EnhancedInputSubsystemInterface.RemoveMappingContext` _returnvalue "/Game/ThirdPerson/Input/IMC_CatInteraction.IMC_CatInteraction" (struct))
        (`EnhancedInputSubsystemInterface.AddMappingContext` _returnvalue "/Game/ThirdPerson/Input/IMC_Interaction.IMC_Interaction" 0 (struct)))
      (`KismetSystemLibrary.Delay` 0.5)
      (`self.K2_DestroyActor`))))

(event `/Game/Blueprints/Interfaces/Interactable.Interact`
  (params (InteractionComponent :type "/Game/Blueprints/Components/InteractionComponent Object Reference"))
  (`parent.Interact` InteractionComponent)
  (`self.Multi_Interact`))

(event `Multi_Interact`
  (`SceneComponent.SetVisibility` (`self.StaticMesh`) true false))

(fn `UserConstructionScript`
  (`parent.UserConstructionScript`))