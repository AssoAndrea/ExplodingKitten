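; Exploding cat actor that produces a bomb when interacted with.
; On BeginPlay, the server takes a free bomb code from KS_GameState and stores it as BombCode.
; Each interaction spawns a BP_Bomb far out in the world, snaps it to the BombSpawn component, then passes it the code and a reference to the cat.
; It also prints the bomb's description as a string.
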(event `self.ReceiveBeginPlay`
  (`parent.ReceiveBeginPlay`)
  (if (`KismetSystemLibrary.IsServer`)
    (bind _asks_game_state (cast `/Game/Blueprints/KS_GameState` (`GameplayStatics.GetGameState`)))
    (bind _code (`/Game/Blueprints/KS_GameState.GetFreeBombCode` _asks_game_state))
    (set `self.BombCode` (break `/Game/Blueprints/Structures/BombCode` _code))))

(event `self.OnInteraction`
  (params (InteractionComponent :type "/Game/Blueprints/Components/InteractionComponent Object Reference"))
  (`parent.OnInteraction` InteractionComponent)
  (bind _returnvalue (`|SpawnActorFromClass` "/Game/Blueprints/Actors/BP_Bomb.BP_Bomb_C" (`KismetMathLibrary.MakeTransform` (0.0 0.0 900000000.0)) "AlwaysSpawn" "MultiplyWithRoot" null null))
  (`self.K2_AttachToComponent` _returnvalue (`self.BombSpawn`) "None" "SnapToTarget" "SnapToTarget" "KeepRelative" true)
  (set `/Game/Blueprints/Actors/BP_Bomb.Code` (`self.BombCode`) _returnvalue)
  (`KismetSystemLibrary.PrintString` (`/Game/Blueprints/Actors/BP_Bomb.GetBombAsString` _returnvalue))
  (set `/Game/Blueprints/Actors/BP_Bomb.Cat` self _returnvalue))

(fn `UserConstructionScript`
  (`parent.UserConstructionScript`))