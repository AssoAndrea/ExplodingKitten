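; BP_Bomb is a bomb actor with a keypad of buttons for entering a numeric code.
; On BeginPlay the authority spawns an attached BP_Button at each Cube socket, using socket names to set digit values or mark OK and NO buttons.
; Pressed numbers append to CurrentCode and print, with no code check here.
; An unconnected debug chain would print each player state's OwnedCodes.
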(event `self.ReceiveBeginPlay`
  (`/Engine/EditorBlueprintResources/ActorMacros.Switch Has Authority`
    (:`Authority`
      (`self.Server_SpawnButtons`))))

(event `Server_SpawnButtons`
  (`self.SpawnButtons`))

(event `SpawnButtons`
  (bind _cube (`self.Cube`))
  (for _array_element (`SceneComponent.GetAllSocketNames` _cube)
    (`|ExecutionSequence`
      (:`then_0`
        (bind _returnvalue (`|SpawnActorFromClass` "/Game/Blueprints/Actors/BP_Button.BP_Button_C" (`SceneComponent.GetSocketTransform` _cube _array_element "RTS_World") "Undefined" "MultiplyWithRoot" null null))
        (`self.K2_AttachToActor` _returnvalue self "None" "KeepWorld" "SnapToTarget" "KeepWorld" true)
        (set `/Game/Blueprints/Actors/BP_Button.OwnerBomb` self _returnvalue))
      (:`then_1`
        (switch `name` _array_element
          (:`Default`
            (set `/Game/Blueprints/Actors/BP_Button.ButtonValue` (`KismetStringLibrary.Conv_StringToInt` (`KismetStringLibrary.Conv_NameToString` _array_element)) _returnvalue)
            (`/Game/Blueprints/Actors/BP_Button.Init` _returnvalue))
          (:`OK`
            (set `/Game/Blueprints/Actors/BP_Button.IsOkButton` true _returnvalue)
            (set `/Game/Blueprints/Actors/BP_Button.IsSpecialButton` true _returnvalue))
          (:`NO`
            (set `/Game/Blueprints/Actors/BP_Button.IsSpecialButton` false _returnvalue)))))))

(event `OnBombNumberPressed`
  (params (Number :type Integer))
  (`KismetArrayLibrary.Array_Add` (`self.CurrentCode`) Number)
  (`KismetSystemLibrary.PrintString` (`KismetStringLibrary.Conv_IntToString` Number)))

(fn `UserConstructionScript`)