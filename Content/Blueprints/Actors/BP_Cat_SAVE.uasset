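; AI cat character that wanders the level, can be scared, and can be picked up by a player for inspection.
; An event-driven Idle/Walking/Scared state machine uses per-state durations and radii, random navmesh destinations and config-driven random animations.
; Scaring triggers a jump and faster move to a random point, ignoring the stored scare origin.
; Multicast-named events toggle movement, gravity and collision for pickup and release, swapping local input contexts on pickup.
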(event `ScareTheCat`
  (params (OriginPoint :type "Vector Structure"))
  (set `self.ScareOriginPoint` OriginPoint)
  (`self.OnForceChangeState` "NewEnumerator1"))

(event `ScaredStateEvent`
  ;[1 1 1] ScaredEvent
  (bind _output_get (set `self.CurrentStatus` "NewEnumerator1"))
  (set `CharacterMovementComponent.MaxWalkSpeed` 300.0 (`self.CharacterMovement`))
  (`self.Jump`)
  (`self.Roam Around` 0.0 (`.StateSearchingRadius_4_CDC8615A43EE6D43CF3666A09AE381DA` (break `/Game/Blueprints/Structures/StateConfigurations` (`BlueprintMapLibrary.Map_Find` (`self.StatusDurations`) _output_get)))))

(event `Roam Around`
  (params (DelayDuration :type "Float (double-precision)") (Radius :type "Float (double-precision)") (Origin :type "Vector Structure"))
  ;[1 1 1] Moving Function
  (if (== Origin (0.0 0.0 0.0))
    (`|AIMoveTo` self (`NavigationSystemV1.K2_GetRandomReachablePointInRadius` (`self.K2_GetActorLocation`) Radius (`self.NavData`) "/Script/NavigationSystem.RecastFilter_UseDefaultArea") null 120.0
      (:`OnSuccess`
        (`self.IdleStateEvent` :!label _label))
      (:`OnFail`
        (`self.WalkingState` :!label _label_2)))
    (else
      (`|AIMoveTo` self Origin null 120.0
        (:`OnSuccess`
          (goto _label))
        (:`OnFail`
          (if (`|EnumEquality` (`self.CurrentStatus`) "NewEnumerator1")
            (`self.ScaredStateEvent`)
            (else
              (goto _label_2))))))))

(event `IdleStateEvent`
  ;[1 1 1] IdleState
  (set `CharacterMovementComponent.MaxWalkSpeed` 200.0 (`self.CharacterMovement`))
  (bind _output_get (set `self.CurrentStatus` "NewEnumerator0"))
  (`self.SetAnimationToPlay` _output_get)
  (`KismetSystemLibrary.Delay` (break `/Game/Blueprints/Structures/StateConfigurations` (`BlueprintMapLibrary.Map_Find` (`self.StatusDurations`) _output_get)))
  (`self.WalkingState`))

(event `WalkingState`
  ;[1 1 1] WalkingState
  (bind _output_get (set `self.CurrentStatus` "NewEnumerator2"))
  (`self.SetAnimationToPlay` _output_get)
  (bind _value (`BlueprintMapLibrary.Map_Find` (`self.StatusDurations`) _output_get))
  (`self.Roam Around` (break `/Game/Blueprints/Structures/StateConfigurations` _value) (`.StateSearchingRadius_4_CDC8615A43EE6D43CF3666A09AE381DA` (break `/Game/Blueprints/Structures/StateConfigurations` _value))))

(event `self.ReceiveBeginPlay`
  ;[1 1 1] BeginPlay
  (bind _returnvalue (`GameplayStatics.GetActorOfClass` "/Script/NavigationSystem.RecastNavMesh"))
  (set `self.NavData` _returnvalue)
  (`self.IdleStateEvent`))

(event `OnForceChangeState`
  (params (NewState :type "/Game/Blueprints/Structures/KittenStatus Enum" :default "NewEnumerator0"))
  ;[1 1 1] ForceChangeState
  (bind _output_get (set `self.CurrentStatus` NewState))
  (switch `/Game/Blueprints/Structures/KittenStatus` _output_get
    (:`NewEnumerator0`
      (`self.IdleStateEvent`))
    (:`NewEnumerator1`
      (`self.ScaredStateEvent`))
    (:`NewEnumerator2`
      (`self.WalkingState`))))

(event `UseCat`
  (params (Controller :type "/Game/Blueprints/KS_PlayerController Object Reference"))
  (`EnhancedInputSubsystemInterface.AddMappingContext` (pcsubsystem `EnhancedInputLocalPlayerSubsystem` Controller) "/Game/ThirdPerson/Input/IMC_CatInteraction.IMC_CatInteraction" 0 (struct)))

(event `self.Interact`
  (params (InteractionComponent :type "/Game/Blueprints/Components/InteractionComponent Object Reference"))
  (`self.Multi_DisableCat` InteractionComponent))

(event `Multi_DisableCat`
  (params (InteractionComp :type "/Game/Blueprints/Components/InteractionComponent Object Reference"))
  (bind _charactermovement (`self.CharacterMovement`))
  (set `CharacterMovementComponent.GravityScale` 0.0 _charactermovement)
  (`/Game/Blueprints/Components/InteractionComponent.InspectObject` InteractionComp self (`self.Inspect Rotation`))
  (`CharacterMovementComponent.DisableMovement` _charactermovement)
  (`PrimitiveComponent.SetCollisionEnabled` (`self.CapsuleComponent`) "NoCollision")
  (bind _aspawn (cast `Pawn` (`ActorComponent.GetOwner` InteractionComp)))
  (bind _asplayer_controller (cast `PlayerController` (`self.GetController` _aspawn)))
  (if (`Controller.IsLocalController` _asplayer_controller)
    (bind _returnvalue (pcsubsystem `EnhancedInputLocalPlayerSubsystem` _asplayer_controller))
    (`EnhancedInputSubsystemInterface.RemoveMappingContext` _returnvalue "/Game/ThirdPerson/Input/IMC_Interaction.IMC_Interaction" (struct))
    (`EnhancedInputSubsystemInterface.AddMappingContext` _returnvalue "/Game/ThirdPerson/Input/IMC_CatInteraction.IMC_CatInteraction" 0 (struct))))

(event `EnableCat`
  (`self.Multi_EnableCat`))

(event `Multi_EnableCat`
  (bind _charactermovement (`self.CharacterMovement`))
  (set `CharacterMovementComponent.GravityScale` 1.0 _charactermovement)
  (`CharacterMovementComponent.SetMovementMode` _charactermovement "MOVE_Walking" 0)
  (`self.K2_DetachFromActor` "KeepWorld" "KeepWorld" "KeepWorld")
  (`PrimitiveComponent.SetCollisionEnabled` (`self.CapsuleComponent`) "QueryAndPhysics"))

(fn `SetAnimationToPlay`
  (params (inStatus :type "/Game/Blueprints/Structures/KittenStatus Enum (by ref)"))
  (bind _config_animationconfiguration (break `/Game/Blueprints/Structures/KittenConfigurationStruct` (`/Game/Blueprints/Structures/KittensConfigurationAssetClass.Config` (`self.KittenConfig`))))
  (bind _value (`BlueprintMapLibrary.Map_Find` _config_animationconfiguration inStatus))
  (`SkeletalMeshComponent.PlayAnimation` (`self.Mesh`) (`|GetArrayItem` (break `/Game/Blueprints/Structures/AnimationArray` _value) (`KismetMathLibrary.RandomInteger` (`KismetArrayLibrary.Array_Length` (break `/Game/Blueprints/Structures/AnimationArray` _value)))) true)
  (return))

(fn `UserConstructionScript`)