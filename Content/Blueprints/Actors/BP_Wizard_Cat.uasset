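; BP_Wizard_Cat is a usable cat actor that opens a portal when a player uses it.
; Its UseCat event calls the parent, then the server spawns a BP_Portal 500 units ahead of the controlled pawn.
; After a short delay the cat destroys itself, and a local controller's Enhanced Input context switches from cat interaction back to standard interaction.
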(event `self.UseCat`
  (params (Controller :type "/Game/Blueprints/KS_PlayerController Object Reference"))
  (bind _returnvalue (`Controller.K2_GetPawn` Controller))
  (bind _returnvalue_2 (pcsubsystem `EnhancedInputLocalPlayerSubsystem` Controller))
  (`parent.UseCat` Controller)
  (`|ExecutionSequence`
    (:`then_0`
      (if (`KismetSystemLibrary.IsServer`)
        (`|SpawnActorFromClass` "/Game/Blueprints/Actors/BP_Portal.BP_Portal_C" (`KismetMathLibrary.MakeTransform` (+ (`self.K2_GetActorLocation` _returnvalue) (* (`self.GetActorForwardVector` _returnvalue) 500.0))) "Undefined" "MultiplyWithRoot" null null)))
    (:`then_1`
      (`KismetSystemLibrary.Delay` 0.2)
      (`self.K2_DestroyActor`)
      (if (`Controller.IsLocalController` Controller)
        (`EnhancedInputSubsystemInterface.RemoveMappingContext` _returnvalue_2 "/Game/ThirdPerson/Input/IMC_CatInteraction.IMC_CatInteraction" (struct))
        (`EnhancedInputSubsystemInterface.AddMappingContext` _returnvalue_2 "/Game/ThirdPerson/Input/IMC_Interaction.IMC_Interaction" 0 (struct))))))

(fn `UserConstructionScript`
  (`parent.UserConstructionScript`))