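; BP_CatFallback is a cat character that wanders the navmesh and can be picked for inspection through interaction.
; It alternates between a timed waiting state and AI moves to random reachable points, with per-status durations and search radii; failed moves retry without waiting.
; Each status change loops a random animation from KittenConfig.
; Interacting disables its gravity, movement and capsule collision and passes it to the InteractionComponent's InspectObject.
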(event `self.ReceiveBeginPlay`
  (bind _output_get (set `self.CurrentStatus` "NewEnumerator0"))
  (`self.SetAnimationToPlay` _output_get)
  (bind _returnvalue (`GameplayStatics.GetActorOfClass` "/Script/NavigationSystem.RecastNavMesh"))
  (set `self.NavData` _returnvalue)
  (`KismetSystemLibrary.Delay` (break `/Game/Blueprints/Structures/StateConfigurations` (`BlueprintMapLibrary.Map_Find` (`self.StatusDurations`) (`self.CurrentStatus`))))
  (bind _output_get_2 (set `self.CurrentStatus` "NewEnumerator2"))
  (`self.SetAnimationToPlay` _output_get_2)
  (`self.Roam Araund`))

(event `Roam Araund`
  (bind _value (`BlueprintMapLibrary.Map_Find` (`self.StatusDurations`) (`self.CurrentStatus`)))
  (`|AIMoveTo` self (`NavigationSystemV1.K2_GetRandomReachablePointInRadius` (`self.K2_GetActorLocation`) (`.StateSearchingRadius_4_CDC8615A43EE6D43CF3666A09AE381DA` (break `/Game/Blueprints/Structures/StateConfigurations` _value)) (`self.NavData`) "/Script/NavigationSystem.RecastFilter_UseDefaultArea") null 120.0
    (:`OnSuccess`
      (bind _output_get (set `self.CurrentStatus` "NewEnumerator0"))
      (`self.SetAnimationToPlay` _output_get)
      (`KismetSystemLibrary.Delay` (break `/Game/Blueprints/Structures/StateConfigurations` _value)))
    (:`OnFail`
      _))
  (bind _output_get_2 (set `self.CurrentStatus` "NewEnumerator2"))
  (`self.SetAnimationToPlay` _output_get_2)
  (`self.Roam Araund`))

(event `self.Interact`
  (params (InteractionComponent :type "/Game/Blueprints/Components/InteractionComponent Object Reference"))
  (`self.OnInteraction` InteractionComponent))

(fn `OnInteraction`
  (params (InteractionComponent :type "/Game/Blueprints/Components/InteractionComponent Object Reference"))
  (bind _charactermovement (`self.CharacterMovement`))
  (set `CharacterMovementComponent.GravityScale` 0.0 _charactermovement)
  (`/Game/Blueprints/Components/InteractionComponent.InspectObject` InteractionComponent self (`self.Inspect Rotation`))
  (`CharacterMovementComponent.DisableMovement` _charactermovement)
  (`PrimitiveComponent.SetCollisionEnabled` (`self.CapsuleComponent`) "NoCollision"))

(fn `SetAnimationToPlay`
  (params (inStatus :type "/Game/Blueprints/Structures/KittenStatus Enum (by ref)"))
  (bind _config_animationconfiguration (break `/Game/Blueprints/Structures/KittenConfigurationStruct` (`/Game/Blueprints/Structures/KittensConfigurationAssetClass.Config` (`self.KittenConfig`))))
  (bind _value (`BlueprintMapLibrary.Map_Find` _config_animationconfiguration inStatus))
  (`SkeletalMeshComponent.PlayAnimation` (`self.Mesh`) (`|GetArrayItem` (break `/Game/Blueprints/Structures/AnimationArray` _value) (`KismetMathLibrary.RandomInteger` (`KismetArrayLibrary.Array_Length` (break `/Game/Blueprints/Structures/AnimationArray` _value)))) true)
  (return))

(fn `UserConstructionScript`)